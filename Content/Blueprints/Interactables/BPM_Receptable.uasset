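; Interactable receptacle that accepts a required item from the player's inventory and tracks whether it has been satisfied.
; Interact finds NeedItem, async-loads and spawns its actor at the Scene transform, optionally showing it, locking collision and consuming it, then calls EventSuccess.
; A missing item triggers a fail sound and temporary message.
; The Still_Placed? timer wiring is disconnected, so removal is only rechecked on interaction.
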(event OnComponentBeginOverlap(CollisionSphere)
  (params (OverlappedComponent :type Primitive%20Component%20Object%20Reference) (OtherActor :type Actor%20Object%20Reference) (OtherComp :type Primitive%20Component%20Object%20Reference) (OtherBodyIndex :type Integer) (bFromSweep :type Boolean) (SweepResult :type Hit%20Result%20Structure%20%28by%20ref%29)))

(event OnComponentEndOverlap(CollisionSphere)
  (params (OverlappedComponent :type Primitive%20Component%20Object%20Reference) (OtherActor :type Actor%20Object%20Reference) (OtherComp :type Primitive%20Component%20Object%20Reference) (OtherBodyIndex :type Integer)))

(event Custom|Still_Placed?
  (if (not (Utilities|IsValid (Variables|References|GetItem%20Ref)))
    (Variables|Default|SetSuccess? false)))

(event EventBeginPlay
  (|CallParentFunction))

(event Collision|EventActorBeginOverlap
  (params (OtherActor :type Actor%20Object%20Reference))
  (|CallParentFunction OtherActor))

(event EventTick
  (params (DeltaSeconds :type Float%20%28single-precision%29))
  (|CallParentFunction DeltaSeconds))

(event EventInteract
  (params (As%20BP%20Main%20Character :type BP%20Main%20Character%20Object%20Reference))
  (bind _scene_transform_in (Variables|Scene|GetScene_Transform_In))
  (if (Variables|NeedItem|GetNeed_Item?)
    (if (Variables|Default|GetSuccess?)
      (if (Utilities|IsValid (Variables|References|GetItem%20Ref))
        (Variables|Default|SetSuccess? true :!label _label)
        (else
          (Variables|Default|SetSuccess? false)
          (bind (_success_ _slot_index _actor_class) (Default|FindItem (Variables|/Game/Blueprints/Bases/Main/Characters/BP_Main_Character.BP_Main_Character_C|GetBPC_Inventory (stale _asbp_main_character)) (Variables|NeedItem|GetNeed%20Item) :!label _label_2))
          (if _success_
            (bind _class (Utilities|AsyncLoadClassAsset _actor_class)
              (:Completed
                (bind _asactor (Utilities|Casting|CastToActorClass _class))
                (Variables|Default|SetItem_To_Spawn _asactor)
                (bind _output_get (Variables|Scene|SetScene_Transform_Out (Math|Transform|MakeTransform (Transformation|GetWorldLocation (Variables|Default|GetScene)) (.rotation _scene_transform_in) (.scale _scene_transform_in))))
                (bind _returnvalue (Game|SpawnActorfromClass (Variables|Default|GetItem_To_Spawn) (Math|Transform|MakeTransform (.Location (Math|Transform|BreakTransform _output_get)) (.Rotation (Math|Transform|BreakTransform _output_get)) (.Scale (Math|Transform|BreakTransform _output_get))) "Undefined" "MultiplyWithRoot" 0 0))
                (Rendering|SetActorHiddenInGame _returnvalue true)
                (Utilities|FlowControl|Delay 0.2)
                (bind _output_get_2 (Variables|References|SetItem%20Ref _returnvalue))
                (if (Variables|NeedItem|GetCan_Place_Item?)
                  (Rendering|SetActorHiddenInGame _output_get_2 false)
                  (if (Variables|NeedItem|GetCan_Take?)
                    _
                    (else
                      (Collision|SetActorEnableCollision (Variables|References|GetItem%20Ref) false))))
                (Variables|Default|SetSuccess? true)
                (if (Variables|NeedItem|GetPersistent_Inventory_Item)
                  _
                  (else
                    (Default|DecrementSlotAmount (Variables|/Game/Blueprints/Bases/Main/Characters/BP_Main_Character.BP_Main_Character_C|GetBPC_Inventory (stale _asbp_main_character)) _slot_index 1)))))
            (else
              (Audio|PlaySoundatLocation (Variables|Default|GetFail_Sound) (Transformation|GetWorldLocation (Variables|Default|GetStaticMesh)) "0, 0, 0" 1.0 1.0 0.0 0 0 0 0)
              (Variables|Default|SetInteraction_Message (Variables|Default|GetObject_Message))
              (Utilities|FlowControl|Delay 1.5)
              (Variables|Default|SetInteraction_Message "")))))
      (else
        (bind _asbp_main_character (Utilities|Casting|CastToBP_Main_Character (Game|GetPlayerCharacter 0)))
        (goto _label_2)))
    (else
      (goto _label)))
  (CallFunction|EventSuccess))

(fn ConstructionScript
  (bind _sphere (Variables|Default|GetSphere))
  (bind _scene (Variables|Default|GetScene))
  (bind _scene_transform_in (Variables|Scene|GetScene_Transform_In))
  (bind _returnvalue (Transformation|GetWorldLocation _scene))
  (bind (_x _y _z) (Math|Vector|BreakVector _returnvalue))
  (|CallParentFunction)
  (Variables|Scene|SetBase_Position (Math|Vector|MakeVector (* _x -1.0) (* _y -1.0) _z))
  (bind _output_get (Variables|Scene|SetScene_Transform_Out (Math|Transform|MakeTransform (+ (.location _scene_transform_in) _returnvalue) (.rotation _scene_transform_in) (.scale _scene_transform_in))))
  (Transformation|SetRelativeTransform (Variables|Default|GetScene) _output_get false false)
  (if (Variables|Scene|GetScene_Debug)
    (Rendering|SetVisibility _sphere true false)
    (else
      (Rendering|SetVisibility _sphere false false))))

(fn EventSuccess
  (return (Variables|Default|GetSuccess?)))