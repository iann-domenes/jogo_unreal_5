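; Lockable table with two drawers that can each hold a configurable item, opened or closed through the parent class's success event.
; BeginPlay spawns each drawer's item and attaches it so it moves with the drawer.
; Interaction uses the player character's line trace to pick the drawer, then slides it on a Timeline with sound, guarded by CanOpen.
; The construction script positions both item spawn points and toggles their debug spheres.
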(event Custom|Interact_Table
  (params (Can_Open? :type Boolean))
  (if Can_Open?
    (bind _asbp_main_character (Utilities|Casting|CastToBP_Main_Character (Game|GetPlayerCharacter 0)))
    (if (Variables|Default|GetCan_Open?)
      (Variables|Default|SetCan_Open? false)
      (bind _hitcomponent (Default|LineTrace _asbp_main_character))
      (bind _asstatic_mesh_component (Utilities|Casting|CastToStaticMeshComponent _hitcomponent))
      (Variables|Default|SetAs%20Static%20Mesh%20Component _asstatic_mesh_component)
      (if (Utilities|String|StartsWith (Utilities|GetObjectName _asstatic_mesh_component) "Static")
        (Variables|Default|SetCan_Open? true)
        (elif (Math|Float|NearlyEqual(Float) (.y (Variables|/Script/Engine.SceneComponent|GetRelativeLocation (Variables|Default|GetAs%20Static%20Mesh%20Component))) 0.0 1e+01)
          (Audio|PlaySoundatLocation (Variables|Default|GetDrawer_Open) (Transformation|GetWorldLocation (Variables|Default|GetStaticMesh)) "0, 0, 0" 1.0 1.0 0.0 0 0 0 0)
          (bind _drawer_location (Timeline|Timeline PlayFromStart)
            (:Update
              (Transformation|SetRelativeLocation (Variables|Default|GetAs%20Static%20Mesh%20Component) (Math|Vector|MakeVector (.x (Variables|/Script/Engine.SceneComponent|GetRelativeLocation (Variables|Default|GetAs%20Static%20Mesh%20Component))) (Math|Float|Lerp 0.0 5e+01 _drawer_location) (.z (Variables|/Script/Engine.SceneComponent|GetRelativeLocation (Variables|Default|GetAs%20Static%20Mesh%20Component)))) false false))
            (:Finished
              (Variables|Default|SetCan_Open? true)))
          (else
            (Audio|PlaySoundatLocation (Variables|Default|GetDrawer_Close) (Transformation|GetWorldLocation (Variables|Default|GetStaticMesh)) "0, 0, 0" 1.0 1.0 0.0 0 0 0 0)
            (Timeline|Timeline Reverse)))))))

(event EventBeginPlay
  (bind _scene_transform_l_in (Variables|Drawers|Drawer_L|GetScene_Transform_L_In))
  (bind _scene_transform_r_in (Variables|Drawers|Drawer_R|GetScene_Transform_R_In))
  (|CallParentFunction)
  (Utilities|FlowControl|Sequence
    (:then_0
      (if (!= (Variables|Drawers|Drawer_R|GetItem_In_Drawer_R) 0)
        (Utilities|FlowControl|Delay 0.2)
        (bind _output_get (Variables|Drawers|Drawer_R|SetScene_Transform_R_Out (Math|Transform|MakeTransform (Variables|/Script/Engine.SceneComponent|GetRelativeLocation (Variables|Default|GetScene_R)) (.rotation _scene_transform_r_in) (.scale _scene_transform_r_in))))
        (bind _returnvalue (Game|SpawnActorfromClass (Variables|Drawers|Drawer_R|GetItem_In_Drawer_R) (Math|Transform|MakeTransform (.Location (Math|Transform|BreakTransform _output_get)) (.Rotation (Math|Transform|BreakTransform _output_get)) (.Scale (Math|Transform|BreakTransform _output_get))) "Undefined" "MultiplyWithRoot" 0 0))
        (Utilities|FlowControl|Delay 0.2)
        (bind _output_get_2 (Variables|Drawers|Drawer_R|SetItem_In_Ref_R _returnvalue))
        (Transformation|AttachComponentToComponent (Variables|/Script/Engine.Actor|GetRootComponent _output_get_2) (Variables|Default|GetDrawer_R) "None" "KeepRelative" "KeepRelative" "KeepWorld" true)))
    (:then_1
      (if (!= (Variables|Drawers|Drawer_L|GetItem_In_Drawer_L) 0)
        (Utilities|FlowControl|Delay 0.2)
        (bind _output_get_3 (Variables|Drawers|Drawer_L|SetScene_Transform_L_Out (Math|Transform|MakeTransform (Variables|/Script/Engine.SceneComponent|GetRelativeLocation (Variables|Default|GetScene_L)) (.rotation _scene_transform_l_in) (.scale _scene_transform_l_in))))
        (bind _returnvalue_2 (Game|SpawnActorfromClass (Variables|Drawers|Drawer_L|GetItem_In_Drawer_L) (Math|Transform|MakeTransform (.Location (Math|Transform|BreakTransform _output_get_3)) (.Rotation (Math|Transform|BreakTransform _output_get_3)) (.Scale (Math|Transform|BreakTransform _output_get_3))) "Undefined" "MultiplyWithRoot" 0 0))
        (Utilities|FlowControl|Delay 0.2)
        (bind _output_get_4 (Variables|Drawers|Drawer_L|SetItem_In_Ref_L _returnvalue_2))
        (Transformation|AttachComponentToComponent (Variables|/Script/Engine.Actor|GetRootComponent _output_get_4) (Variables|Default|GetDrawer_L) "None" "KeepRelative" "KeepRelative" "KeepWorld" true)))))

(event Collision|EventActorBeginOverlap
  (params (OtherActor :type Actor%20Object%20Reference))
  (|CallParentFunction OtherActor) ; This node is disabled and will not be called.\nDrag off pins to build functionality.
)

(event EventTick
  (params (DeltaSeconds :type Float%20%28single-precision%29))
  (|CallParentFunction DeltaSeconds) ; This node is disabled and will not be called.\nDrag off pins to build functionality.
)

(fn ConstructionScript
  (bind _scene_r (Variables|Default|GetScene_R))
  (bind _scene_transform_r_in (Variables|Drawers|Drawer_R|GetScene_Transform_R_In))
  (bind _sphere_r (Variables|Default|GetSphere_R))
  (bind _scene_transform_l_in (Variables|Drawers|Drawer_L|GetScene_Transform_L_In))
  (bind _scene_l (Variables|Default|GetScene_L))
  (bind _sphere_l (Variables|Default|GetSphere_L))
  (bind _returnvalue (Transformation|GetWorldLocation _scene_l))
  (bind _returnvalue_2 (Transformation|GetWorldLocation _scene_r))
  (bind (_x _y _z) (Math|Vector|BreakVector _returnvalue))
  (bind (_x_2 _y_2 _z_2) (Math|Vector|BreakVector _returnvalue_2))
  (|CallParentFunction)
  (Variables|Drawers|Drawer_R|SetBase_Position_R (Math|Vector|MakeVector (* _x_2 -1.0) (* _y_2 -1.0) _z_2))
  (bind _output_get (Variables|Drawers|Drawer_R|SetScene_Transform_R_Out (Math|Transform|MakeTransform (+ (.location _scene_transform_r_in) _returnvalue_2) (.rotation _scene_transform_r_in) (.scale _scene_transform_r_in))))
  (Transformation|SetRelativeTransform (Variables|Default|GetScene_R) _output_get false false)
  (if (Variables|Drawers|Drawer_R|GetScene_Debug_R)
    (Rendering|SetVisibility _sphere_r true false)
    (else
      (Rendering|SetVisibility _sphere_r false false)))
  (Variables|Drawers|Drawer_L|SetBase_Position_L (Math|Vector|MakeVector (* _x -1.0) (* _y -1.0) _z))
  (bind _output_get_2 (Variables|Drawers|Drawer_L|SetScene_Transform_L_Out (Math|Transform|MakeTransform (+ (.location _scene_transform_l_in) _returnvalue) (.rotation _scene_transform_l_in) (.scale _scene_transform_l_in))))
  (Transformation|SetRelativeTransform (Variables|Default|GetScene_L) _output_get_2 false false)
  (if (Variables|Drawers|Drawer_L|GetScene_Debug_L)
    (Rendering|SetVisibility _sphere_l true false)
    (else
      (Rendering|SetVisibility _sphere_l false false))))

(fn EventSuccess
  (bind _success_ (|CallParentFunction))
  (CallFunction|InteractTable _success_)
  (return _success_))