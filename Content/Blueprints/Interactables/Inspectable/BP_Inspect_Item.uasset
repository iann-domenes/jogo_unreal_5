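; Temporary inspection actor that shows an item for examination or a readable note, taking input from the character until Interact ends it.
; Inspect and ReadNote create their widgets; setter events set the item mesh's initial rotation and scale.
; Mouse axes rotate the mesh, the wheel zooms via clamped SceneCapture2D FOV, and right-click resets both.
; Q toggles note text through render opacity, with InNote blocking rotation and zoom while it shows.
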(event Custom|Set_Inspection_Rotation
  (params (Item_Rotation :type Rotator))
  (bind _item (Variables|Default|GetItem))
  (bind _returnvalue (Transformation|GetWorldTransform _item))
  ;[1 1 1] Set Inspection Rotation Dinamically
  (bind _output_get (Variables|Default|SetInitial%20Rotation Item_Rotation))
  (Transformation|SetWorldTransform _item (Math|Transform|MakeTransform (.location _returnvalue) _output_get (.scale _returnvalue)) false false))

(event Custom|Set_Inspect_Scale
  (params (Inspection_Scale :type Vector))
  (bind _item (Variables|Default|GetItem))
  (bind _returnvalue (Transformation|GetWorldTransform _item))
  ;[1 1 1] Set Inspection Scale Dinamically
  (Transformation|SetWorldTransform _item (Math|Transform|MakeTransform (.location _returnvalue) (.rotation _returnvalue) Inspection_Scale) false false))

(event Input|EnhancedActionEvents|EnhancedInputActionIA_Interact
  (params (ActionValue :type Vector%202D%20Structure) (ElapsedSeconds :type Float%20%28double-precision%29) (TriggeredSeconds :type Float%20%28double-precision%29) (InputAction :type Input%20Action%20Object%20Reference :default "/Game/Input/Default/Actions/IA_Interact.IA_Interact"))
  (bind _returnvalue (Game|GetPlayerController 0))
  ;[1 1 1] Quit inspection
  (:Completed
    (Input|DisableInput _returnvalue)
    (Input|EnableInput (Variables|Default|GetCharacter) _returnvalue)
    (Utilities|IsValid (Variables|Default|GetInspect_Widget_Ref)
      (:Is%20Valid
        (Widget|RemovefromParent (Variables|Default|GetInspect_Widget_Ref))
        (Variables|Default|SetInspect_Widget_Ref 0)
        (Actor|DestroyActor)
        (Utilities|IsValid (Variables|Default|GetNote_Widget_Reference)
          (:Is%20Valid
            (Widget|RemovefromParent (Variables|Default|GetNote_Widget_Reference))
            (Variables|Default|SetNote_Widget_Reference 0)
            (Actor|DestroyActor)))))))

(event EventBeginPlay
  (|CallParentFunction) ; This node is disabled and will not be called.\nDrag off pins to build functionality.
)

(event Collision|EventActorBeginOverlap
  (params (OtherActor :type Actor%20Object%20Reference))
  (|CallParentFunction OtherActor) ; This node is disabled and will not be called.\nDrag off pins to build functionality.
)

(event EventTick
  (params (DeltaSeconds :type Float%20%28single-precision%29))
  (|CallParentFunction DeltaSeconds) ; This node is disabled and will not be called.\nDrag off pins to build functionality.
)

(event EventInspect
  (params (Character :type BP%20Main%20Character%20Object%20Reference) (Inspected_Item :type Static%20Mesh%20Object%20Reference) (Item_Name :type Text) (Item_Description :type Text))
  (bind _returnvalue (Game|GetPlayerController 0))
  ;[1 1 1] Event Inspect
  (Variables|Default|SetCharacter Character)
  (Components|StaticMesh|SetStaticMesh (Variables|Default|GetItem) Inspected_Item)
  (bind _returnvalue_2 (UserInterface|CreateWidget "/Game/Widgets/Inspect/W_Inspect.W_Inspect_C" 0 Item_Name Item_Description))
  (bind _output_get (Variables|Default|SetInspect_Widget_Ref _returnvalue_2))
  (UserInterface|Viewport|AddtoViewport _output_get 0)
  (Input|DisableInput (Variables|Default|GetCharacter) _returnvalue)
  (Input|EnableInput _returnvalue)
  (Variables|Default|SetRotate? true))

(event EventReadNote
  (params (Character :type BP%20Main%20Character%20Object%20Reference) (Note_Text :type Text))
  (bind _returnvalue (Game|GetPlayerController 0))
  ;[1 1 1] Event Read Note
  (Variables|Default|SetCharacter Character)
  (bind _returnvalue_2 (UserInterface|CreateWidget "/Game/Widgets/Inspect/Note/W_Note.W_Note_C" 0 Note_Text))
  (bind _output_get (Variables|Default|SetNote_Widget_Reference _returnvalue_2))
  (UserInterface|Viewport|AddtoViewport _output_get 0)
  (Input|DisableInput (Variables|Default|GetCharacter) _returnvalue)
  (Input|EnableInput _returnvalue))

(event Input|MouseEvents|MouseX
  (params (AxisValue :type Float%20%28single-precision%29))
  ;[1 1 1] Mouse movement while inspecting item
  ;;[0.05286 0.05286 0.05286] Set Mouse Movement Horizontally
  (if (not (Variables|Default|GetIn_Note?))
    (if (Variables|Default|GetRotate?)
      (Transformation|SetWorldRotation (Variables|Default|GetItem) (Math|Rotator|CombineRotators (Transformation|GetWorldRotation (Variables|Default|GetItem)) (Math|Rotator|MakeRotator 0.0 0.0 (* AxisValue -3.0))) false false))))

(event Input|MouseEvents|MouseY
  (params (AxisValue :type Float%20%28single-precision%29))
  ;[1 1 1] Mouse movement while inspecting item
  ;;[0.05286 0.05286 0.05286] Set Mouse Movement Vertically
  (if (not (Variables|Default|GetIn_Note?))
    (if (Variables|Default|GetRotate?)
      (Transformation|SetWorldRotation (Variables|Default|GetItem) (Math|Rotator|CombineRotators (Transformation|GetWorldRotation (Variables|Default|GetItem)) (Math|Rotator|MakeRotator 0.0 (* AxisValue -3.0) 0.0)) false false))))

(event Input|MouseEvents|LeftMouseButton
  (params (Key :type Key%20Structure :default "None"))
  ;[1 1 1] Mouse movement while inspecting item
  ;;[1 1 1] Allow to rotate
)

(event Input|MouseEvents|RightMouseButton
  (params (Key :type Key%20Structure :default "None"))
  ;[1 1 1] Mouse movement while inspecting item
  ;;[1 1 1] Resetting Transform os Inspected Item
  (:Pressed
    (if (not (Variables|Default|GetIn_Note?))
      (Transformation|SetWorldRotation (Variables|Default|GetItem) (Variables|Default|GetInitial%20Rotation) false false)
      (Variables|/Script/Engine.SceneCaptureComponent2D|SetFOVAngle (Variables|Default|GetSceneCaptureComponent2D) 5e+01))))

(event Input|MouseEvents|MouseWheelUp
  (params (Key :type Key%20Structure :default "None"))
  (bind _scenecapturecomponent2d (Variables|Default|GetSceneCaptureComponent2D))
  ;[1 1 1] Mouse movement while inspecting item
  ;;[0.05286 0.05286 0.05286 0] Zoom In
  (:Pressed
    (if (not (Variables|Default|GetIn_Note?))
      (Variables|/Script/Engine.SceneCaptureComponent2D|SetFOVAngle _scenecapturecomponent2d (Math|Float|Clamp(Float) (- (Variables|/Script/Engine.SceneCaptureComponent2D|GetFOVAngle _scenecapturecomponent2d) 3.0) 3e+01 8e+01)))))

(event Input|KeyboardEvents|Q
  (params (Key :type Key%20Structure :default "None"))
  (bind _note_widget_reference (Variables|Default|GetNote_Widget_Reference))
  (bind _read_text_q (Variables|/Game/Widgets/Inspect/Note/W_Note.W_Note_C|GetRead_Text_Q _note_widget_reference))
  ;[1 1 1] Press [Q] Key to Read Note
  (:Pressed
    (Variables|Default|GetNote_Widget_Reference
      (:then
        (bind _isa (Utilities|FlowControl|FlipFlop)
          (:A
            (Variables|Default|SetIs%20A _isa)
            (Widget|SetRenderOpacity (Variables|/Game/Widgets/Inspect/Note/W_Note.W_Note_C|GetNote_Canvas_Panel _note_widget_reference) 1.0)
            (Widget|SetRenderOpacity _read_text_q 0.0)
            (Variables|Default|SetIs%20A false)
            (Variables|Default|SetIn_Note? true))
          (:B
            (Widget|SetRenderOpacity (Variables|/Game/Widgets/Inspect/Note/W_Note.W_Note_C|GetNote_Canvas_Panel (Variables|Default|GetNote_Widget_Reference)) 0.0)
            (Widget|SetRenderOpacity _read_text_q 1.0)
            (Variables|Default|SetIn_Note? false))))
      (:else))))

(event Input|MouseEvents|MouseWheelDown
  (params (Key :type Key%20Structure :default "None"))
  (bind _scenecapturecomponent2d (Variables|Default|GetSceneCaptureComponent2D))
  ;[1 1 1] Mouse movement while inspecting item
  ;;[0.05286 0.05286 0.05286] Zoom Out
  (:Pressed
    (if (not (Variables|Default|GetIn_Note?))
      (Variables|/Script/Engine.SceneCaptureComponent2D|SetFOVAngle _scenecapturecomponent2d (Math|Float|Clamp(Float) (+ (Variables|/Script/Engine.SceneCaptureComponent2D|GetFOVAngle _scenecapturecomponent2d) 3.0) 3e+01 8e+01)))))

(fn ConstructionScript
  (|CallParentFunction))