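; BP_Battery is an interactable battery pickup that recharges the player's flashlight.
; It caches the main character on BeginPlay, and Interact adds a fixed charge, clamped to the maximum, then destroys the battery if the current charge is at or below a threshold.
; Otherwise it briefly shows one of two messages on the player text widget, depending on whether the inventory component finds a Flashlight.
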(event EventBeginPlay
  (|CallParentFunction)
  (bind _asbp_main_character (Utilities|Casting|CastToBP_Main_Character (Game|GetPlayerCharacter 0)))
  (Variables|Default|SetAs%20BP%20Main%20Character_0 _asbp_main_character))

(event Collision|EventActorBeginOverlap
  (params (OtherActor :type Actor%20Object%20Reference))
  (|CallParentFunction OtherActor) ; This node is disabled and will not be called.\nDrag off pins to build functionality.
)

(event EventTick
  (params (DeltaSeconds :type Float%20%28single-precision%29))
  (|CallParentFunction DeltaSeconds) ; This node is disabled and will not be called.\nDrag off pins to build functionality.
)

(event EventInteract
  (params (As%20BP%20Main%20Character :type BP%20Main%20Character%20Object%20Reference))
  (bind _as_bp_main_character_0 (Variables|Default|GetAs%20BP%20Main%20Character_0))
  (bind _as_bp_main_character_0_2 (Variables|Default|GetAs%20BP%20Main%20Character_0))
  (bind _player_text_widget (Variables|/Game/Blueprints/Bases/Main/Characters/BP_Main_Character.BP_Main_Character_C|GetPlayer_Text_Widget _as_bp_main_character_0_2))
  (bind _player_text_widget_2 (Variables|/Game/Blueprints/Bases/Main/Characters/BP_Main_Character.BP_Main_Character_C|GetPlayer_Text_Widget _as_bp_main_character_0_2))
  (if (<= (Variables|/Game/Blueprints/Bases/Main/Characters/BP_Main_Character.BP_Main_Character_C|GetFlashlight_Charge _as_bp_main_character_0) 4e+01)
    (Variables|/Game/Blueprints/Bases/Main/Characters/BP_Main_Character.BP_Main_Character_C|SetFlashlight_Charge _as_bp_main_character_0 (Math|Float|Clamp(Float) (+ (Variables|/Game/Blueprints/Bases/Main/Characters/BP_Main_Character.BP_Main_Character_C|GetFlashlight_Charge _as_bp_main_character_0) 75.0) 0.0 (Variables|/Game/Blueprints/Bases/Main/Characters/BP_Main_Character.BP_Main_Character_C|GetMax_Flashlight_Charge _as_bp_main_character_0)))
    (Actor|DestroyActor)
    (else
      (bind _success_ (Default|FindItem (Variables|/Game/Blueprints/Bases/Main/Characters/BP_Main_Character.BP_Main_Character_C|GetBPC_Inventory (Variables|Default|GetAs%20BP%20Main%20Character_0)) "Flashlight"))
      (if _success_
        (Variables|/Game/Widgets/Inventory/W_Item_Name_Description.W_Item_Name_Description_C|SetPlayer_Text _player_text_widget (Variables|Default|GetObject_Message))
        (Utilities|FlowControl|Delay 1.5)
        (Variables|/Game/Widgets/Inventory/W_Item_Name_Description.W_Item_Name_Description_C|SetPlayer_Text _player_text_widget "")
        (else
          (Variables|/Game/Widgets/Inventory/W_Item_Name_Description.W_Item_Name_Description_C|SetPlayer_Text _player_text_widget_2 (Variables|Default|GetText_Message))
          (Utilities|FlowControl|Delay 1.5)
          (Variables|/Game/Widgets/Inventory/W_Item_Name_Description.W_Item_Name_Description_C|SetPlayer_Text _player_text_widget_2 ""))))))

(fn ConstructionScript
  (|CallParentFunction))