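; BP_Lighter is a lighter actor with a point light, a candle particle and a mesh, whose light intensity animates while the player's FlashlightOn flag is set.
; It caches BP_Main_Character on BeginPlay, then Tick plays a timeline that lerps the light between minimum and maximum intensity.
; A helper function disables the mesh's collision.
; The logic that shows the flame and turns off the mesh's shadow is unconnected and never runs.
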(event EventBeginPlay
  (|CallParentFunction)
  (bind _asbp_main_character (Utilities|Casting|CastToBP_Main_Character (Game|GetPlayerCharacter 0)))
  (Variables|Default|SetAs%20BP%20Main%20Character_0 _asbp_main_character))

(event Collision|EventActorBeginOverlap
  (params (OtherActor :type Actor%20Object%20Reference))
  (|CallParentFunction OtherActor) ; This node is disabled and will not be called.\nDrag off pins to build functionality.
)

(event EventTick
  (params (DeltaSeconds :type Float%20%28single-precision%29))
  (|CallParentFunction DeltaSeconds)
  (if (Variables|/Game/Blueprints/Bases/Main/Characters/BP_Main_Character.BP_Main_Character_C|GetFlashlight_On? (Variables|Default|GetAs%20BP%20Main%20Character_0))
    (bind _light_intensity (Timeline|Timeline Play)
      (:Update
        (Rendering|Components|Light|SetIntensity (Variables|Default|GetPointLight) (Math|Float|Lerp (Variables|Default|GetMin_Intensity) (Variables|Default|GetMax_Intensity) _light_intensity))))))

(fn ConstructionScript
  (|CallParentFunction))

(fn DisableColision
  (Collision|SetCollisionEnabled (Variables|Default|GetSM_Lighter) "NoCollision"))