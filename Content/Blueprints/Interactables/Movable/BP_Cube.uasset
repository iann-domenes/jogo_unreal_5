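; BP_Cube is a movable interactable cube that the main character can push or pull.
; Overlapping its FWD component shows a HUD prompt and sets CanMovableInteract on the character.
; While the character is interacting, Tick reads its movement axes and calls Move_Direction, printing debug messages.
; Move_Direction interpolates the mesh's relative location without sweep, using its right vector for forward/back and forward vector for left/right.
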(event OnComponentBeginOverlap(FWD)
  (params (OverlappedComponent :type Primitive%20Component%20Object%20Reference) (OtherActor :type Actor%20Object%20Reference) (OtherComp :type Primitive%20Component%20Object%20Reference) (OtherBodyIndex :type Integer) (bFromSweep :type Boolean) (SweepResult :type Hit%20Result%20Structure%20%28by%20ref%29))
  (Class|BPIHUD|ShowInteractionMessage(Message) (HUD|GetHUD (Game|GetPlayerController 0)) "mover")
  (Variables|/Game/Blueprints/Bases/Main/Characters/BP_Main_Character.BP_Main_Character_C|SetCan_Movable_Interact (Variables|Default|GetCharacter_Ref) true))

(event OnComponentEndOverlap(FWD)
  (params (OverlappedComponent :type Primitive%20Component%20Object%20Reference) (OtherActor :type Actor%20Object%20Reference) (OtherComp :type Primitive%20Component%20Object%20Reference) (OtherBodyIndex :type Integer))
  (Class|BPIHUD|HideInteractionMessage(Message) (HUD|GetHUD (Game|GetPlayerController 0)))
  (Variables|/Game/Blueprints/Bases/Main/Characters/BP_Main_Character.BP_Main_Character_C|SetCan_Movable_Interact (Variables|Default|GetCharacter_Ref) false))

(event EventBeginPlay
  (bind _returnvalue (Actor|GetActorOfClass "/Game/Blueprints/Bases/Main/Characters/BP_Main_Character.BP_Main_Character_C"))
  (Variables|Default|SetCharacter_Ref _returnvalue))

(event Collision|EventActorBeginOverlap
  (params (OtherActor :type Actor%20Object%20Reference)))

(event EventTick
  (params (DeltaSeconds :type Float%20%28single-precision%29))
  (bind _character_ref (Variables|Default|GetCharacter_Ref))
  (bind _character_ref_2 (Variables|Default|GetCharacter_Ref))
  (bind _forward_backward_axis (Variables|/Game/Blueprints/Bases/Main/Characters/BP_Main_Character.BP_Main_Character_C|GetForward_Backward_Axis _character_ref_2))
  (bind _left_right_axis (Variables|/Game/Blueprints/Bases/Main/Characters/BP_Main_Character.BP_Main_Character_C|GetLeft_Right_Axis _character_ref_2))
  (if (Variables|/Game/Blueprints/Bases/Main/Characters/BP_Main_Character.BP_Main_Character_C|GetIs_Movable_Interacting? _character_ref)
    (if (Variables|/Game/Blueprints/Bases/Main/Characters/BP_Main_Character.BP_Main_Character_C|GetCan_Movable_Interact _character_ref)
      (Utilities|FlowControl|Sequence
        (:then_0
          (if (== _forward_backward_axis 0.0)
            (Development|PrintString "NOT forword or back" true true "(R=1.000000,G=0.100299,B=0.817294,A=1.000000)" 2.0 "5569")
            (elif (>= _forward_backward_axis 0.1)
              (Development|PrintString "Move Forward" true true "(R=0.305721,G=0.225796,B=1.000000,A=1.000000)" 2.0 "8545457")
              (Utilities|MoveDirection true -3e+01)
              (else
                (Development|PrintString "Moving Back" true true "(R=0.645398,G=1.000000,B=0.470796,A=1.000000)" 2.0 "854")
                (Utilities|MoveDirection true 3e+01)))))
        (:then_1
          (if (== _left_right_axis 0.0)
            (Development|PrintString "NOT forword or back" true true "(R=1.000000,G=0.100299,B=0.817294,A=1.000000)" 2.0 "00502")
            (elif (>= _left_right_axis 0.1)
              (Development|PrintString "Moving rIGHT" true true "(R=0.305721,G=0.225796,B=1.000000,A=1.000000)" 2.0 "565899")
              (Utilities|MoveDirection false 3e+01)
              (else
                (Development|PrintString "Moving Left" true true "(R=0.645398,G=1.000000,B=0.470796,A=1.000000)" 2.0 "5568748")
                (Utilities|MoveDirection false -3e+01)))))))))

(fn ConstructionScript)

(fn GetInteractionMessage
  (return ""))

(fn GetObjectMessage
  (return ""))