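; A lockable interactable door that cycles through closed, part-open and open states, swinging away from or toward either side by yaw rotation.
; The parent's EventSuccess result feeds Interact_Door as its Locked flag, which must be true for the door to move.
; When closed, a camera-to-box dot product picks the swing direction.
; Each step plays a sound and a shared timeline, with a DoOnce blocking re-triggers until it finishes.
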(event Custom|Interact_Door
  (params (Locked? :type Boolean))
  ;[1 1 1] Checking wich side of the Door the Player is when its Closed
  (bind _asbp_main_character (Utilities|Casting|CastToBP_Main_Character (Game|GetPlayerCharacter 0)))
  (Variables|Default|SetAs%20BP%20Main%20Character_0_0_0 _asbp_main_character)
  (if (Variables|Default|GetClosed?)
    (if (> (Math|Vector|DotProduct (Math|Vector|GetForwardVector (Variables|/Game/Blueprints/Bases/Main/Characters/BP_Main_Character.BP_Main_Character_C|GetFollowCamera (Variables|Default|GetAs%20BP%20Main%20Character_0_0_0))) (Math|Vector|GetForwardVector (Variables|Default|GetBox_Collision self))) 0.0)
      (Variables|Default|SetDoor_Open_Side 1.0)
      (else
        (Variables|Default|SetDoor_Open_Side -1.0))))
  (if Locked?
    (Utilities|FlowControl|DoOnce false :!label _label
      (:Completed
        ;[1 1 1] Setting door states variables
        (switch Utilities|FlowControl|Switch|SwitchonEN_Door_States (Variables|Default|GetEN_Door_States)
          (:NewEnumerator0
            (Variables|Default|SetEN_Door_States "NewEnumerator1")
            (Variables|Default|SetPart_Open? true)
            (Variables|Default|SetClosed? false)
            (Variables|Default|SetOpen? true)
            ;[1 1 1] Sound Effect
            (Audio|PlaySoundatLocation (Variables|Default|GetPart_Open) (Transformation|GetWorldLocation (Variables|Default|GetDoor)) "0, 0, 0" 1.0 1.0 0.0 0 0 0 0)
            (bind (_direction _part_open _open _close) (Timeline|Door_Animation PlayFromStart)
              (:Update
                ;[1 1 1] Setting Relative Rotation of the Door
                (switch Utilities|FlowControl|Switch|SwitchonEN_Door_States (Variables|Default|GetEN_Door_States)
                  (:NewEnumerator0
                    (Transformation|SetRelativeRotation (Variables|Default|GetDoor) (Math|Rotator|MakeRotator 0.0 0.0 (* _close (Variables|Default|GetDoor_Open_Side))) false false))
                  (:NewEnumerator1
                    (Transformation|SetRelativeRotation (Variables|Default|GetDoor) (Math|Rotator|MakeRotator 0.0 0.0 (* _part_open (Variables|Default|GetDoor_Open_Side))) false false))
                  (:NewEnumerator2
                    (Transformation|SetRelativeRotation (Variables|Default|GetDoor) (Math|Rotator|MakeRotator 0.0 0.0 (* _open (Variables|Default|GetDoor_Open_Side))) false false))))
              (:Finished
                (goto _label Reset))))
          (:NewEnumerator1
            (Variables|Default|SetEN_Door_States "NewEnumerator2")
            (Variables|Default|SetPart_Open? false)
            (Variables|Default|SetClosed? false)
            (Variables|Default|SetOpen? true)
            (Audio|PlaySoundatLocation (Variables|Default|GetOpen) (Transformation|GetWorldLocation (Variables|Default|GetDoor)) "0, 0, 0" 1.0 1.0 0.0 0 0 0 0)
            (Timeline|Door_Animation PlayFromStart))
          (:NewEnumerator2
            (Variables|Default|SetEN_Door_States "NewEnumerator0")
            (Variables|Default|SetPart_Open? false)
            (Variables|Default|SetClosed? true)
            (Variables|Default|SetOpen? false)
            (Audio|PlaySoundatLocation (Variables|Default|GetClose) (Transformation|GetWorldLocation (Variables|Default|GetDoor)) "0, 0, 0" 1.0 1.0 0.0 0 0 0 0)
            (Timeline|Door_Animation PlayFromStart)))))))

(event EventBeginPlay
  (|CallParentFunction) ; This node is disabled and will not be called.\nDrag off pins to build functionality.
)

(event Collision|EventActorBeginOverlap
  (params (OtherActor :type Actor%20Object%20Reference))
  (|CallParentFunction OtherActor) ; This node is disabled and will not be called.\nDrag off pins to build functionality.
)

(event EventTick
  (params (DeltaSeconds :type Float%20%28single-precision%29))
  (|CallParentFunction DeltaSeconds) ; This node is disabled and will not be called.\nDrag off pins to build functionality.
)

(fn ConstructionScript
  (|CallParentFunction)
  (Components|StaticMesh|SetStaticMesh (Variables|Default|GetStaticMesh) (Variables|Default|GetDoor_Frame_Mesh))
  (Components|StaticMesh|SetStaticMesh (Variables|Default|GetDoor) (Variables|Default|GetDoor_Mesh)))

(fn EventSuccess
  (bind _success_ (|CallParentFunction))
  (CallFunction|InteractDoor _success_)
  (return _success_))