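; Interactable wall gap that the player squeezes through from either end, with proximity icons on each side.
; Interact shrinks the capsule, locks look input, fades, teleports to that side's start arrow and switches to its camera.
; Tick offsets that camera and spotlight from the follow camera and picks single-node squeeze animations by speed.
; Leaving the matching exit box fades, moves the player to a leave arrow and restores normal control.
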(event OnComponentEndOverlap(BoxCollisionOne)
  (params (OverlappedComponent :type Primitive%20Component%20Object%20Reference) (OtherActor :type Actor%20Object%20Reference) (OtherComp :type Primitive%20Component%20Object%20Reference) (OtherBodyIndex :type Integer))
  (bind _as_bp_main_character (Variables|References|GetAs%20BP%20Main%20Character))
  (bind _leavearrowone (Variables|Default|GetLeaveArrowOne))
  (bind _as_bp_main_character_2 (Variables|References|GetAs%20BP%20Main%20Character))
  (bind _returnvalue (Transformation|GetWorldTransform _leavearrowone))
  (bind _charactermovement (Variables|/Script/Engine.Character|GetCharacterMovement _as_bp_main_character_2))
  (if (== OtherActor (Game|GetPlayerCharacter 0))
    (if (Variables|Camera|GetIs_In_First_Cam?)
      (Utilities|FlowControl|DoOnce false :!label _label
        (:Completed
          (CallFunction|FadeCamera (Game|GetPlayerCameraManager 0) 0.3 2.0 0.5)
          (Utilities|FlowControl|Delay 0.5)
          (Pawn|Components|CharacterMovement|DisableMovement (Variables|/Script/Engine.Character|GetCharacterMovement _as_bp_main_character))
          (Variables|/Game/Blueprints/Bases/Main/Characters/BP_Main_Character.BP_Main_Character_C|SetIs_In_Gap _as_bp_main_character false)
          (Components|Capsule|SetCapsuleRadius (Variables|/Script/Engine.Character|GetCapsuleComponent _as_bp_main_character) 35.0 true)
          (Audio|PlaySoundatLocation 0 (Transformation|GetActorLocation (Variables|References|GetAs%20BP%20Main%20Character)) "0, 0, 0" 1.0 1.0 0.0 0 0 0 0)
          (Rendering|SetVisibility (Variables|Default|GetSpotLightOne) false false)
          (Transformation|SetWorldTransform (Variables|/Script/Engine.Actor|GetRootComponent (Variables|References|GetAs%20BP%20Main%20Character)) (Math|Transform|MakeTransform (.location _returnvalue) (.rotation _returnvalue) "1.000000,1.000000,1.000000") false false)
          (Input|SetIgnoreLookInput (Game|GetPlayerController 0) false)
          (Components|Animation|SetAnimationMode (Variables|/Script/Engine.Character|GetMesh (Variables|References|GetAs%20BP%20Main%20Character)) "AnimationBlueprint" true)
          (Pawn|Components|CharacterMovement|SetMovementMode _charactermovement (Variables|/Script/Engine.CharacterMovementComponent|GetDefaultLandMovementMode _charactermovement) 0)
          (Variables|Camera|SetIs_In_First_Cam? false)
          (Game|Player|SetViewTargetwithBlend (Game|GetPlayerController 0) (Variables|References|GetAs%20BP%20Main%20Character) 0.0 "VTBlend_Linear" 0.0 false)
          (goto _label Reset))))))

(event OnComponentBeginOverlap(InnerSphereCollisionTwo)
  (params (OverlappedComponent :type Primitive%20Component%20Object%20Reference) (OtherActor :type Actor%20Object%20Reference) (OtherComp :type Primitive%20Component%20Object%20Reference) (OtherBodyIndex :type Integer) (bFromSweep :type Boolean) (SweepResult :type Hit%20Result%20Structure%20%28by%20ref%29))
  ;[1 1 1] Interact Icon
  ;;[1 1 1] Two
  (if (== OtherActor (Game|GetPlayerCharacter 0))
    (Rendering|SetVisibility (Variables|Default|GetInnerInteractIconTwo) true false)
    (Rendering|SetVisibility (Variables|Default|GetOuterInteractIconTwo) false false)))

(event OnComponentEndOverlap(InnerSphereCollisionTwo)
  (params (OverlappedComponent :type Primitive%20Component%20Object%20Reference) (OtherActor :type Actor%20Object%20Reference) (OtherComp :type Primitive%20Component%20Object%20Reference) (OtherBodyIndex :type Integer))
  ;[1 1 1] Interact Icon
  ;;[1 1 1] Two
  (if (== (Game|GetPlayerCharacter 0) OtherActor)
    (Rendering|SetVisibility (Variables|Default|GetInnerInteractIconTwo) false false)
    (Rendering|SetVisibility (Variables|Default|GetOuterInteractIconTwo) true false)))

(event OnComponentBeginOverlap(OutherSphereCollisionTwo)
  (params (OverlappedComponent :type Primitive%20Component%20Object%20Reference) (OtherActor :type Actor%20Object%20Reference) (OtherComp :type Primitive%20Component%20Object%20Reference) (OtherBodyIndex :type Integer) (bFromSweep :type Boolean) (SweepResult :type Hit%20Result%20Structure%20%28by%20ref%29))
  ;[1 1 1] Interact Icon
  ;;[1 1 1] Two
  (if (== OtherActor (Game|GetPlayerCharacter 0))
    (Rendering|SetVisibility (Variables|Default|GetOuterInteractIconTwo) true false)))

(event OnComponentEndOverlap(OutherSphereCollisionTwo)
  (params (OverlappedComponent :type Primitive%20Component%20Object%20Reference) (OtherActor :type Actor%20Object%20Reference) (OtherComp :type Primitive%20Component%20Object%20Reference) (OtherBodyIndex :type Integer))
  ;[1 1 1] Interact Icon
  ;;[1 1 1] Two
  (if (== (Game|GetPlayerCharacter 0) OtherActor)
    (Rendering|SetVisibility (Variables|Default|GetOuterInteractIconTwo) false false)))

(event OnComponentEndOverlap(BoxCollisionTwo)
  (params (OverlappedComponent :type Primitive%20Component%20Object%20Reference) (OtherActor :type Actor%20Object%20Reference) (OtherComp :type Primitive%20Component%20Object%20Reference) (OtherBodyIndex :type Integer))
  (bind _as_bp_main_character (Variables|References|GetAs%20BP%20Main%20Character))
  (bind _as_bp_main_character_2 (Variables|References|GetAs%20BP%20Main%20Character))
  (bind _leavearrowtwo (Variables|Default|GetLeaveArrowTwo))
  (bind _returnvalue (Transformation|GetWorldTransform _leavearrowtwo))
  (bind _charactermovement (Variables|/Script/Engine.Character|GetCharacterMovement _as_bp_main_character))
  (if (== 0 (Game|GetPlayerCharacter 0))
    (if (Variables|Camera|GetIs_In_Second_Cam?)
      (Utilities|FlowControl|DoOnce false :!label _label
        (:Completed
          (CallFunction|FadeCamera (Game|GetPlayerCameraManager 0) 0.3 2.0 0.5)
          (Utilities|FlowControl|Delay 0.5)
          (Pawn|Components|CharacterMovement|DisableMovement (Variables|/Script/Engine.Character|GetCharacterMovement _as_bp_main_character_2))
          (Variables|/Game/Blueprints/Bases/Main/Characters/BP_Main_Character.BP_Main_Character_C|SetIs_In_Gap _as_bp_main_character_2 false)
          (Components|Capsule|SetCapsuleRadius (Variables|/Script/Engine.Character|GetCapsuleComponent _as_bp_main_character_2) 35.0 true)
          (Audio|PlaySoundatLocation 0 (Transformation|GetActorLocation (Variables|References|GetAs%20BP%20Main%20Character)) "0, 0, 0" 1.0 1.0 0.0 0 0 0 0)
          (Rendering|SetVisibility (Variables|Default|GetSpotLightTwo) false false)
          (Transformation|SetWorldTransform (Variables|/Script/Engine.Actor|GetRootComponent (Variables|References|GetAs%20BP%20Main%20Character)) (Math|Transform|MakeTransform (.location _returnvalue) (.rotation _returnvalue) "1.000000,1.000000,1.000000") false false)
          (Input|SetIgnoreLookInput (Game|GetPlayerController 0) false)
          (Components|Animation|SetAnimationMode (Variables|/Script/Engine.Character|GetMesh (Variables|References|GetAs%20BP%20Main%20Character)) "AnimationBlueprint" true)
          (Pawn|Components|CharacterMovement|SetMovementMode _charactermovement (Variables|/Script/Engine.CharacterMovementComponent|GetDefaultLandMovementMode _charactermovement) 0)
          (Variables|Camera|SetIs_In_Second_Cam? false)
          (Game|Player|SetViewTargetwithBlend (Game|GetPlayerController 0) (Variables|References|GetAs%20BP%20Main%20Character) 0.0 "VTBlend_Linear" 0.0 false)
          (goto _label Reset))))))

(event OnComponentBeginOverlap(OuterSphereCollisionOne)
  (params (OverlappedComponent :type Primitive%20Component%20Object%20Reference) (OtherActor :type Actor%20Object%20Reference) (OtherComp :type Primitive%20Component%20Object%20Reference) (OtherBodyIndex :type Integer) (bFromSweep :type Boolean) (SweepResult :type Hit%20Result%20Structure%20%28by%20ref%29))
  ;[1 1 1] Interact Icon
  ;;[1 1 1] One
  (if (== OtherActor (Game|GetPlayerCharacter 0))
    (Rendering|SetVisibility (Variables|Default|GetOuterInteractIconOne) true false)))

(event OnComponentEndOverlap(OuterSphereCollisionOne)
  (params (OverlappedComponent :type Primitive%20Component%20Object%20Reference) (OtherActor :type Actor%20Object%20Reference) (OtherComp :type Primitive%20Component%20Object%20Reference) (OtherBodyIndex :type Integer))
  ;[1 1 1] Interact Icon
  ;;[1 1 1] One
  (if (== (Game|GetPlayerCharacter 0) OtherActor)
    (Rendering|SetVisibility (Variables|Default|GetOuterInteractIconOne) false false)))

(event OnComponentBeginOverlap(InnerSphereCollisionOne)
  (params (OverlappedComponent :type Primitive%20Component%20Object%20Reference) (OtherActor :type Actor%20Object%20Reference) (OtherComp :type Primitive%20Component%20Object%20Reference) (OtherBodyIndex :type Integer) (bFromSweep :type Boolean) (SweepResult :type Hit%20Result%20Structure%20%28by%20ref%29))
  ;[1 1 1] Interact Icon
  ;;[1 1 1] One
  (if (== OtherActor (Game|GetPlayerCharacter 0))
    (Rendering|SetVisibility (Variables|Default|GetInnerInteractIconOne) true false)
    (Rendering|SetVisibility (Variables|Default|GetOuterInteractIconOne) false false)))

(event OnComponentEndOverlap(InnerSphereCollisionOne)
  (params (OverlappedComponent :type Primitive%20Component%20Object%20Reference) (OtherActor :type Actor%20Object%20Reference) (OtherComp :type Primitive%20Component%20Object%20Reference) (OtherBodyIndex :type Integer))
  ;[1 1 1] Interact Icon
  ;;[1 1 1] One
  (if (== (Game|GetPlayerCharacter 0) OtherActor)
    _))

(event Custom|CustomEvent
  (params (OverlappedComponent :type Primitive%20Component%20Object%20Reference) (OtherActor :type Actor%20Object%20Reference) (OtherComp :type Primitive%20Component%20Object%20Reference) (OtherBodyIndex :type Integer)))

(event Custom|Fade_Camera
  (params (Camera_Manager :type Player%20Camera%20Manager%20Object%20Reference) (Start_Fase_Time :type Float%20%28single-precision%29) (Duration_Between :type Float%20%28single-precision%29) (End_Fade_Time :type Float%20%28single-precision%29))
  ;[1 1 1] Camera Fade
  (CameraFades|StartCameraFade :self Camera_Manager :ToAlpha 1.0 :Duration Start_Fase_Time :bHoldWhenFinished true)
  (Utilities|FlowControl|Delay Duration_Between)
  (CameraFades|StartCameraFade :self Camera_Manager :FromAlpha 1.0 :ToAlpha 0.0 :Duration End_Fade_Time))

(event EventBeginPlay
  ;[1 1 1] Begin Play
  (bind _asbp_main_character (Utilities|Casting|CastToBP_Main_Character (Game|GetPlayerCharacter 0)))
  (Variables|References|SetAs%20BP%20Main%20Character _asbp_main_character))

(event EventTick
  (params (DeltaSeconds :type Float%20%28single-precision%29))
  (bind _as_bp_main_character (Variables|References|GetAs%20BP%20Main%20Character))
  (bind _as_bp_main_character_2 (Variables|References|GetAs%20BP%20Main%20Character))
  (bind _as_bp_main_character_3 (Variables|References|GetAs%20BP%20Main%20Character))
  (bind _followcamera (Variables|/Game/Blueprints/Bases/Main/Characters/BP_Main_Character.BP_Main_Character_C|GetFollowCamera _as_bp_main_character))
  (bind _mesh (Variables|/Script/Engine.Character|GetMesh _as_bp_main_character_2))
  (bind _mesh_2 (Variables|/Script/Engine.Character|GetMesh _as_bp_main_character_3))
  (bind _returnvalue (Transformation|GetWorldLocation _followcamera))
  (bind _returnvalue_2 (Transformation|GetWorldLocation _followcamera))
  (bind _returnvalue_3 (- (.y _returnvalue_2) 1e+01))
  (bind _returnvalue_4 (- (.z _returnvalue_2) 1e+01))
  (bind _returnvalue_5 (+ (.x _returnvalue) 1e+01))
  (bind _returnvalue_6 (- (.y _returnvalue) 1e+01))
  ;[1 1 1] Event Tick
  (if (Variables|/Game/Blueprints/Bases/Main/Characters/BP_Main_Character.BP_Main_Character_C|GetIs_In_Gap _as_bp_main_character)
    (if (Variables|Camera|GetIs_In_First_Cam?)
      (Transformation|SetWorldLocation (Variables|Default|GetCameraOne) (Math|Vector|MakeVector (.x _returnvalue) _returnvalue_5 _returnvalue_6) false false)
      (Transformation|SetWorldLocation (Variables|Default|GetSpotLightOne) (Math|Vector|MakeVector (.x _returnvalue) _returnvalue_5 _returnvalue_6) false false)
      (if (> (Math|Vector|VectorLength (Variables|/Script/Engine.MovementComponent|GetVelocity (Variables|/Script/Engine.Character|GetCharacterMovement (Variables|References|GetAs%20BP%20Main%20Character)))) 35.0)
        (Utilities|FlowControl|DoOnce false :!label _label
          (:Completed
            (Components|Animation|PlayAnimation _mesh_2 "/Game/Characters/Mannequins/Animations/UE5_ObstructionAnimation1.UE5_ObstructionAnimation1" true)))
        (else
          (Components|Animation|PlayAnimation _mesh_2 "/Game/Characters/Mannequins/Animations/UE5_ObstructionBeginAnimation.UE5_ObstructionBeginAnimation" true)
          (goto _label Reset)))
      (else
        (Transformation|SetWorldLocation (Variables|Default|GetCameraTwo) (Math|Vector|MakeVector (.x _returnvalue_2) _returnvalue_3 _returnvalue_4) false false)
        (Transformation|SetWorldLocation (Variables|Default|GetSpotLightTwo) (Math|Vector|MakeVector (.x _returnvalue_2) _returnvalue_3 _returnvalue_4) false false)
        (if (> (Math|Vector|VectorLength (Variables|/Script/Engine.MovementComponent|GetVelocity (Variables|/Script/Engine.Character|GetCharacterMovement (Variables|References|GetAs%20BP%20Main%20Character)))) 35.0)
          (Utilities|FlowControl|DoOnce false :!label _label_2
            (:Completed
              (Components|Animation|PlayAnimation _mesh "/Game/Characters/Mannequins/Animations/UE5_ObstructionAnimation1.UE5_ObstructionAnimation1" true)))
          (else
            (Components|Animation|PlayAnimation _mesh "/Game/Characters/Mannequins/Animations/UE5_ObstructionBeginAnimation.UE5_ObstructionBeginAnimation" true)
            (goto _label_2 Reset)))))))

(event EventInteract
  (params (As%20BP%20Main%20Character :type BP%20Main%20Character%20Object%20Reference))
  (bind _charactermovement (Variables|/Script/Engine.Character|GetCharacterMovement As%20BP%20Main%20Character))
  (bind _startarrowtwo (Variables|Default|GetStartArrowTwo))
  (bind _startarrowone (Variables|Default|GetStartArrowOne))
  (bind _returnvalue (Transformation|GetWorldTransform _startarrowtwo))
  (bind _returnvalue_2 (Transformation|GetWorldTransform _startarrowone))
  (bind _charactermovement_2 (Variables|/Script/Engine.Character|GetCharacterMovement (Variables|References|GetAs%20BP%20Main%20Character)))
  (bind _charactermovement_3 (Variables|/Script/Engine.Character|GetCharacterMovement (Variables|References|GetAs%20BP%20Main%20Character)))
  ;[1 1 1] Interaction CamOne
  (if (Collision|IsOverlappingActor (Variables|Default|GetInnerSphereCollisionOne) (Game|GetPlayerCharacter 0) :!class /Script/Engine.PrimitiveComponent)
    (Components|Activation|Activate (Variables|Default|GetCameraOne) false)
    (Components|Capsule|SetCapsuleRadius (Variables|/Script/Engine.Character|GetCapsuleComponent As%20BP%20Main%20Character) 1e+01 true)
    (Pawn|Components|CharacterMovement|DisableMovement _charactermovement)
    (Input|SetIgnoreLookInput (Game|GetPlayerController 0) true)
    (CallFunction|FadeCamera (Game|GetPlayerCameraManager 0) 1.5 2.0 1.5)
    (Utilities|FlowControl|Delay 2.0)
    (Audio|PlaySoundatLocation 0 (Transformation|GetActorLocation (Variables|References|GetAs%20BP%20Main%20Character)) "0, 0, 0" 1.0 1.0 0.0 0 0 0 0)
    (Variables|/Game/Blueprints/Bases/Main/Characters/BP_Main_Character.BP_Main_Character_C|SetIs_In_Gap (Variables|References|GetAs%20BP%20Main%20Character) true)
    (Rendering|SetVisibility (Variables|Default|GetSpotLightOne) true false)
    (Transformation|SetWorldTransform (Variables|/Script/Engine.Actor|GetRootComponent (Variables|References|GetAs%20BP%20Main%20Character)) (Math|Transform|MakeTransform (.location _returnvalue_2) (.rotation _returnvalue_2) "1.000000,1.000000,1.000000") false false)
    (Pawn|SetControlRotation (Game|GetPlayerController 0) (Transformation|GetActorRotation (Game|GetPlayerCharacter 0)))
    (Variables|Camera|SetIs_In_First_Cam? true)
    (Components|Activation|Deactivate (Variables|Default|GetCameraTwo))
    (Game|Player|SetViewTargetwithBlend (Game|GetPlayerController 0) (Components|GetOwner (Variables|Default|GetCameraOne)) 0.0 "VTBlend_Linear" 0.0 false)
    (Components|Animation|SetAnimationMode (Variables|/Script/Engine.Character|GetMesh (Variables|References|GetAs%20BP%20Main%20Character)) "AnimationSingleNode" true)
    (Pawn|Components|CharacterMovement|SetMovementMode _charactermovement_3 (Variables|/Script/Engine.CharacterMovementComponent|GetDefaultLandMovementMode _charactermovement_3) 0)
    (else
      ;[1 1 1] Interaction CamTwo
      (if (Collision|IsOverlappingActor (Variables|Default|GetInnerSphereCollisionTwo) (Game|GetPlayerCharacter 0) :!class /Script/Engine.PrimitiveComponent)
        (Components|Activation|Activate (Variables|Default|GetCameraTwo) false)
        (Components|Capsule|SetCapsuleRadius (Variables|/Script/Engine.Character|GetCapsuleComponent (Variables|References|GetAs%20BP%20Main%20Character)) 1e+01 true)
        (Pawn|Components|CharacterMovement|DisableMovement _charactermovement)
        (Input|SetIgnoreLookInput (Game|GetPlayerController 0) true)
        (CallFunction|FadeCamera (Game|GetPlayerCameraManager 0) 1.5 2.0 1.5)
        (Utilities|FlowControl|Delay 2.0)
        (Audio|PlaySoundatLocation 0 (Transformation|GetActorLocation (Variables|References|GetAs%20BP%20Main%20Character)) "0, 0, 0" 1.0 1.0 0.0 0 0 0 0)
        (Variables|/Game/Blueprints/Bases/Main/Characters/BP_Main_Character.BP_Main_Character_C|SetIs_In_Gap (Variables|References|GetAs%20BP%20Main%20Character) true)
        (Rendering|SetVisibility (Variables|Default|GetSpotLightTwo) true false)
        (Transformation|SetWorldTransform (Variables|/Script/Engine.Actor|GetRootComponent (Variables|References|GetAs%20BP%20Main%20Character)) (Math|Transform|MakeTransform (.location _returnvalue) (.rotation _returnvalue) "1.000000,1.000000,1.000000") false false)
        (Pawn|SetControlRotation (Game|GetPlayerController 0) (Transformation|GetActorRotation (Game|GetPlayerCharacter 0)))
        (Variables|Camera|SetIs_In_Second_Cam? true)
        (Components|Activation|Deactivate (Variables|Default|GetCameraOne))
        (Game|Player|SetViewTargetwithBlend (Game|GetPlayerController 0) (Components|GetOwner (Variables|Default|GetCameraTwo)) 0.0 "VTBlend_Linear" 0.0 false)
        (Components|Animation|SetAnimationMode (Variables|/Script/Engine.Character|GetMesh (Variables|References|GetAs%20BP%20Main%20Character)) "AnimationSingleNode" true)
        (Pawn|Components|CharacterMovement|SetMovementMode _charactermovement_2 (Variables|/Script/Engine.CharacterMovementComponent|GetDefaultLandMovementMode _charactermovement_2) 0)))))

(fn ConstructionScript)

(fn GetInteractionMessage
  (return ""))