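; Base interactable actor that shows a billboard prompt when the player is nearby and looking at it, and supplies an interaction message.
; While the player overlaps CollisionSphere, a looping timer replaces Tick, comparing camera forward with direction to the actor by dot product to toggle the billboard.
; The construction script applies sphere radii, component offsets and debug visibility.
; InteractSphere has no overlap logic here, and billboard-rotation code is unconnected.
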(event OnComponentBeginOverlap(CollisionSphere)
  (params (OverlappedComponent :type Primitive%20Component%20Object%20Reference) (OtherActor :type Actor%20Object%20Reference) (OtherComp :type Primitive%20Component%20Object%20Reference) (OtherBodyIndex :type Integer) (bFromSweep :type Boolean) (SweepResult :type Hit%20Result%20Structure%20%28by%20ref%29))
  (if (== OtherActor (Game|GetPlayerCharacter 0))
    (if (Variables|Transform|GetShow_Billboard?)
      (bind _returnvalue (Utilities|Time|SetTimerbyEvent (delegate Custom|Look) 0.1 true))
      (Variables|Default|SetTimer _returnvalue))))

(event OnComponentEndOverlap(CollisionSphere)
  (params (OverlappedComponent :type Primitive%20Component%20Object%20Reference) (OtherActor :type Actor%20Object%20Reference) (OtherComp :type Primitive%20Component%20Object%20Reference) (OtherBodyIndex :type Integer))
  (if (== (Game|GetPlayerCharacter 0) OtherActor)
    (Utilities|Time|ClearandInvalidateTimerbyHandle (Variables|Default|GetTimer))
    (Rendering|SetVisibility (Variables|Default|GetBillboard) false false)))

(event Custom|Look
  (bind _billboard (Variables|Default|GetBillboard))
  (bind _as_bp_main_character (Variables|Default|GetAs%20BP%20Main%20Character))
  (bind _followcamera (Variables|/Game/Blueprints/Bases/Main/Characters/BP_Main_Character.BP_Main_Character_C|GetFollowCamera _as_bp_main_character))
  (if (>= (Math|Vector|DotProduct (Math|Vector|Normalize (- (Transformation|GetActorLocation) (Transformation|GetWorldLocation _followcamera))) (Math|Vector|GetForwardVector _followcamera)) 0.99)
    (Rendering|SetVisibility _billboard true false)
    (else
      (Rendering|SetVisibility _billboard false false))))

(event EventBeginPlay
  (bind _asbp_main_character (Utilities|Casting|CastToBP_Main_Character (Game|GetPlayerCharacter 0)))
  (Variables|Default|SetAs%20BP%20Main%20Character _asbp_main_character))

(event Collision|EventActorBeginOverlap
  (params (OtherActor :type Actor%20Object%20Reference)))

(event EventTick
  (params (DeltaSeconds :type Float%20%28single-precision%29)))

(fn ConstructionScript
  (bind _billboard (Variables|Default|GetBillboard))
  (bind _collisionsphere (Variables|Default|GetCollisionSphere))
  (bind _interactsphere (Variables|Default|GetInteractSphere))
  (Utilities|FlowControl|Sequence
    (:then_0
      (Components|Sphere|SetSphereRadius (Variables|Default|GetCollisionSphere) (Variables|Transform|GetCollision%20Sphere%20Radius) true)
      (Components|Sphere|SetSphereRadius (Variables|Default|GetInteractSphere) (Variables|Transform|GetInteract%20Sphere%20Radius) true)
      (Transformation|SetRelativeLocation (Variables|Default|GetInteractSphere) (Variables|Transform|GetInteract%20Sphere%20Location) false false)
      (Transformation|SetRelativeLocation (Variables|Default|GetBillboard) (Variables|Transform|GetBillboard_Location) false false))
    (:then_1
      (if (Variables|Transform|GetDebbuging?)
        (Rendering|SetVisibility _collisionsphere true false)
        (Rendering|SetVisibility _billboard true false)
        (Rendering|SetVisibility _interactsphere true false)
        (else
          (Rendering|SetVisibility _collisionsphere false false)
          (Rendering|SetVisibility _billboard false false)
          (Rendering|SetVisibility _interactsphere false false))))))

(fn GetInteractionMessage
  (return (Variables|Text|GetInteraction_Message)))