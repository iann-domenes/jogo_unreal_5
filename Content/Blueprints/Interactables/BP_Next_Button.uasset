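; BP_Next_Button is an interactable that sends the player to the next level.
; On Interact, it saves the player's BPC_Inventory data to SavedInventory on BP_GameInstance.
; It then finds the current level name in the game instance's LevelOrder array and opens the following entry.
; On the last level nothing opens, while an unlisted level leads to the first entry because Find returns -1.
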(event EventBeginPlay
  (|CallParentFunction) ; This node is disabled and will not be called.\nDrag off pins to build functionality.
)

(event Collision|EventActorBeginOverlap
  (params (OtherActor :type Actor%20Object%20Reference))
  (|CallParentFunction OtherActor) ; This node is disabled and will not be called.\nDrag off pins to build functionality.
)

(event EventTick
  (params (DeltaSeconds :type Float%20%28single-precision%29))
  (|CallParentFunction DeltaSeconds) ; This node is disabled and will not be called.\nDrag off pins to build functionality.
)

(event EventInteract
  (params (As%20BP%20Main%20Character :type BP%20Main%20Character%20Object%20Reference))
  (bind _saved_inventory (Default|GetInventoryData (Actor|GetComponentbyClass (Game|GetPlayerCharacter 0) "/Game/Blueprints/Components/BPC_Inventory.BPC_Inventory_C")))
  (bind _asbp_game_instance (Utilities|Casting|CastToBP_GameInstance (Game|GetGameInstance)))
  (Variables|/Game/Maps/BP_GameInstance.BP_GameInstance_C|SetSavedInventory _asbp_game_instance _saved_inventory)
  (bind _returnvalue (Game|GetCurrentLevelName true))
  (bind _asbp_game_instance_2 (Utilities|Casting|CastToBP_GameInstance (Game|GetGameInstance)))
  (if (Utilities|Array|IsValidIndex (Variables|/Game/Maps/BP_GameInstance.BP_GameInstance_C|GetLevelOrder _asbp_game_instance_2) (+ (Utilities|Array|FindItem (Variables|/Game/Maps/BP_GameInstance.BP_GameInstance_C|GetLevelOrder _asbp_game_instance_2) _returnvalue) 1))
    (Game|OpenLevel(byName) (Utilities|String|StringToName (Utilities|Array|Get(acopy) (Variables|/Game/Maps/BP_GameInstance.BP_GameInstance_C|GetLevelOrder _asbp_game_instance_2) (+ (Utilities|Array|FindItem (Variables|/Game/Maps/BP_GameInstance.BP_GameInstance_C|GetLevelOrder _asbp_game_instance_2) _returnvalue) 1))))))

(fn ConstructionScript
  (|CallParentFunction))